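; Snake tail actor that builds a body of spline mesh components along its Spline in the construction script.
; EndMeshSetup adds an X-forward end piece between the first two spline points.
; MidOfSp then adds a Y-forward piece for every segment, including that first one, storing them in the Snak array from index 1.
; The event graph is inert, with Add_Tail left as an empty stub.
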(event Custom|Add_Tail)

(event EventBeginPlay)

(event Collision|EventActorBeginOverlap
  (params (OtherActor :type Actor%20Object%20Reference)))

(event EventTick
  (params (DeltaSeconds :type Float%20%28single-precision%29)))

(fn ConstructionScript
  (CallFunction|EndMeshSetup)
  (CallFunction|MidOfSp))

(fn EndMeshSetup
  (bind _returnvalue (Class|KismetMathLibrary|SignOfInteger))
  (bind _spline (Variables|Default|GetSpline))
  (bind _spline_2 (Variables|Default|GetSpline))
  (bind (_location _tangent) (Spline|GetLocationandTangentatSplinePoint _spline_2 _returnvalue "Local"))
  (bind _returnvalue_2 (+ _returnvalue 1))
  (bind (_location_2 _tangent_2) (Spline|GetLocationandTangentatSplinePoint _spline _returnvalue_2 "Local"))
  (bind _returnvalue_3 (AddComponent|AddSplineMeshComponent false))
  (Utilities|Array|SetArrayElem (Variables|Default|Getsnak) 0 0)
  (SplineMesh|SetForwardAxis _returnvalue_3 "X" true)
  (SplineMesh|SetStartandEnd _returnvalue_3 _location _tangent _location_2 _tangent_2 true :!class /Script/Engine.SplineMeshComponent))

(fn MidOfSp
  (for _index (range 0 (- (Spline|GetNumberOfSplinePoints (Variables|Default|GetSpline)) 2))
    (bind _returnvalue (AddComponent|AddSplineMeshComponent false))
    (Utilities|Array|SetArrayElem (Variables|Default|Getsnak) (+ _index 1) _returnvalue)
    (SplineMesh|SetForwardAxis _returnvalue "Y" true)
    (SplineMesh|SetStartandEnd _returnvalue (.Location (Spline|GetLocationandTangentatSplinePoint (Variables|Default|GetSpline) _index "Local")) (.Tangent (Spline|GetLocationandTangentatSplinePoint (Variables|Default|GetSpline) _index "Local")) (.Location (Spline|GetLocationandTangentatSplinePoint (Variables|Default|GetSpline) (+ _index 1) "Local")) (.Tangent (Spline|GetLocationandTangentatSplinePoint (Variables|Default|GetSpline) (+ _index 1) "Local")) true :!class /Script/Engine.SplineMeshComponent)))